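; Camera actor that takes high-resolution screenshots from its own view through HighResShot console commands.
; Each shot event switches the player's view target to this actor, runs the command, waits briefly, then returns view to the player character.
; CustomShot builds a Saved/Screenshots path from a file ID, with out-of-range sizes falling back to viewport dimensions.
; MidShot uses a fixed ID and half-viewport size; both print their command.
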(event Custom|StartShot
  (Game|Player|SetViewTargetwithBlend (Game|GetPlayerController 0) self 0.0 "VTBlend_Linear" 0.0 false)
  (Development|ExecuteConsoleCommand "HighResShot 1" 0)
  (Utilities|FlowControl|Delay 0.1)
  (Game|Player|SetViewTargetwithBlend (Game|GetPlayerController 0) (Game|GetPlayerCharacter 0) 0.0 "VTBlend_Linear" 0.0 true))

(event Custom|CustomShot
  (params (ShotFileID :type Integer) (Width :type Integer) (Height :type Integer))
  (bind _retwidth (CallFunction|GetClipWidth Width))
  (bind _returnvalue (Class|KismetSystemLibrary|GetProjectSavedDirectory))
  (bind _returnvalue_2 (Utilities|String|ToString(Integer) ShotFileID))
  (bind _retheight (CallFunction|GetClipHeght Height))
  (bind _returnvalue_3 (Utilities|String|ToString(Integer) _retwidth))
  (bind _returnvalue_4 (Utilities|String|ToString(Integer) _retheight))
  (bind _returnvalue_5 (Utilities|String|Append "HighResShot filename=" _returnvalue "Screenshots/" _returnvalue_2 ".png" " " _returnvalue_3 "x" _returnvalue_4 " "))
  (Game|Player|SetViewTargetwithBlend (Game|GetPlayerController 0) self 0.0 "VTBlend_Linear" 0.0 false)
  (Development|ExecuteConsoleCommand _returnvalue_5 0) ; HightResShot filename=xxxx wxh
  (Utilities|FlowControl|Delay 1.0)
  (Game|Player|SetViewTargetwithBlend (Game|GetPlayerController 0) (Game|GetPlayerCharacter 0) 0.0 "VTBlend_Linear" 0.0 true)
  (Development|PrintString _returnvalue_5 true true "(R=0.000000,G=0.660000,B=1.000000,A=1.000000)" 5e+01))

(event Custom|MidShot
  (bind _returnvalue (Class|KismetSystemLibrary|GetProjectSavedDirectory))
  (bind _returnvalue_2 (Utilities|String|ToString(Integer) 10002))
  (bind _returnvalue_3 (Viewport|GetViewportSize))
  (bind (_x _y) (Math|Vector2D|BreakVector2D _returnvalue_3))
  (bind _returnvalue_4 (/ _x 2.0))
  (bind _returnvalue_5 (/ _y 2.0))
  (bind _returnvalue_6 (Class|KismetMathLibrary|FCeil64 _returnvalue_5))
  (bind _returnvalue_7 (Class|KismetMathLibrary|FCeil64 _returnvalue_4))
  (bind _returnvalue_8 (Utilities|String|ToString(Integer) _returnvalue_7))
  (bind _returnvalue_9 (Utilities|String|ToString(Integer) _returnvalue_6))
  (bind _returnvalue_10 (Utilities|String|Append "HighResShot filename=" _returnvalue "Screenshots/" _returnvalue_2 ".png" " " _returnvalue_8 "x" _returnvalue_9 " " " 0 0  " _returnvalue_8 "x" _returnvalue_9 " 0 0 0 1 "))
  (Game|Player|SetViewTargetwithBlend (Game|GetPlayerController 0) self 0.0 "VTBlend_Linear" 0.0 false)
  (Development|ExecuteConsoleCommand _returnvalue_10 0) ; HightResShot filename=xxxx wxh
  (Utilities|FlowControl|Delay 1.0)
  (Game|Player|SetViewTargetwithBlend (Game|GetPlayerController 0) (Game|GetPlayerCharacter 0) 0.0 "VTBlend_Linear" 0.0 true)
  (Development|PrintString _returnvalue_10 true true "(R=0.000000,G=0.660000,B=1.000000,A=1.000000)" 5e+01))

(event EventBeginPlay)

(event Collision|EventActorBeginOverlap
  (params (OtherActor :type Actor%20Object%20Reference)))

(event EventTick
  (params (DeltaSeconds :type Float%20%28single-precision%29)))

(fn ConstructionScript)

(fn GetClipWidth
  (params (Width :type Integer))
  (bind _returnvalue (Viewport|GetViewportSize))
  (bind _x (Math|Vector2D|BreakVector2D _returnvalue))
  (if (or (> Width _x) (< Width 1))
    (return (Math|Float|Truncate _x))
    (else
      (return Width))))

(fn GetClipHeght
  (params (Height :type Integer))
  (bind _returnvalue (Viewport|GetViewportSize))
  (bind _y (Math|Vector2D|BreakVector2D _returnvalue))
  (if (or (> Height _y) (< Height 1))
    (return (Math|Float|Truncate _y))
    (else
      (return Height))))